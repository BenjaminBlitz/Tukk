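; Enemy spawner actor that spawns waves of NPC_Character enemies at its own transform.
; On BeginPlay it binds SpawnEnemy to the TopDownGameMode's respawn-enemy event, so the game mode decides when waves spawn.
; Each call spawns EnnemySpawned NPCs, nudged to avoid collisions but always spawned, then raises that count by EnemyIncrement so waves grow.
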(event Custom|SpawnEnemy
  (for _index (range 0 (- (Variables|Default|GetEnnemySpawned) 1))
    (Game|SpawnActorfromClass "/Game/AI/NPC_Character.NPC_Character_C" (Transformation|GetActorTransform) "AdjustIfPossibleButAlwaysSpawn" 0 0))
  (Variables|Default|SetEnnemySpawned (+ (Variables|Default|GetEnnemySpawned) (Variables|Default|GetEnemyIncrement))))

(event EventBeginPlay
  (bind _astop_down_game_mode (Utilities|Casting|CastToTopDownGameMode (Game|GetGameMode)))
  (EventDispatchers|BindEventtoRespawnEnemy _astop_down_game_mode (delegate Custom|SpawnEnemy)))

(fn ConstructionScript)